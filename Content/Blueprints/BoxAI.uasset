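; BoxAI is a suicide-bomber enemy that patrols between points and chases the player on sight.
; From BeginPlay, PatrolToPoint uses AIMoveTo to loop through PatrolPoints, wrapping the index at the end.
; PawnSensing sets InRange and moves it toward the seen TopDownCharacter.
; Reaching the player spawns an explosion with sound, subtracts health and destroys the box, while a failed chase resumes patrol.
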(event OnSeePawn(PawnSensing)
  (params (Pawn :type Pawn%20Object%20Reference))
  ;[1 1 1] Chase Player
  (Variables|Default|SetInRange true)
  (bind _astop_down_character (Utilities|Casting|CastToTopDownCharacter Pawn))
  (AI|AIMoveTo self "0, 0, 0" _astop_down_character 5.0 false
    (:OnSuccess
      (Effects|SpawnEmitteratLocation "/Game/StarterContent/Particles/P_Explosion.P_Explosion" (Transformation|GetActorLocation _astop_down_character))
      (Audio|PlaySound2D "/Game/StarterContent/Audio/Explosion_Cue.Explosion_Cue")
      (Default|SubtractHealth _astop_down_character (Variables|Default|GetDamage))
      (Actor|DestroyActor))
    (:OnFail
      (CallFunction|PatroltoPoint))))

(event Custom|PatrolToPoint
  ;[1 1 1] Patrolling
  (AI|AIMoveTo self "0, 0, 0" (Utilities|Array|Get(acopy) (Variables|Default|GetPatrolPoints) (Variables|Default|GetPatrolPointIndex)) 5.0 false
    (:OnSuccess
      (if (>= (Variables|Default|GetPatrolPointIndex) (- (Utilities|Array|Length (Variables|Default|GetPatrolPoints)) 1))
        (Variables|Default|SetPatrolPointIndex 0)
        (else
          (Math|Integer|IncrementInt (Variables|Default|GetPatrolPointIndex)
            (:%20%20
              _))))
      (CallFunction|PatroltoPoint))))

(event EventBeginPlay
  (CallFunction|PatroltoPoint))

(fn ConstructionScript)