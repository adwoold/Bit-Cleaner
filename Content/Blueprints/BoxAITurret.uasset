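; BoxAITurret is a stationary enemy turret that shoots at the player on sight and awards score when killed.
; PawnSensing turns it to face the TopDownCharacter and spawns a TestProjectile from ArrowShot, throttled by a Delay-reset flag.
; Damage and healing events adjust AIAttributes health; at zero or below, KillAI adds BitsDropped to the player's score and destroys the turret.
; Patrol logic is present but disconnected, so it never runs.
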(event OnSeePawn(PawnSensing)
  (params (Pawn :type Pawn%20Object%20Reference))
  ;[1 1 1] Chase Player
  (Variables|Default|SetInRange true)
  (bind _astop_down_character (Utilities|Casting|CastToTopDownCharacter Pawn))
  (Utilities|FlowControl|Sequence
    (:then_0
      (Transformation|SetActorRotation (Math|Rotator|FindLookatRotation (Transformation|GetActorLocation) (Transformation|GetActorLocation _astop_down_character))))
    (:then_1
      (if (Variables|Default|GetSpawnProjectile)
        (Game|SpawnActorfromClass "/Game/Characters/Blueprints/TestProjectile.TestProjectile_C" (Transformation|GetWorldTransform (Variables|Default|GetArrowShot)) "Undefined" 0 0)
        (Variables|Default|SetSpawnProjectile false)
        (Utilities|FlowControl|Delay 1.5)
        (Variables|Default|SetSpawnProjectile true)))))

(event Custom|PatrolToPoint
  ;[1 1 1] Patrolling
)

(event EventKillAI
  (params (Dead? :type Boolean))
  ;[1 1 1] Destroy Actor and award score
  (if Dead?
    (bind _astop_down_character (Utilities|Casting|CastToTopDownCharacter (Game|GetPlayerCharacter 0)))
    (Default|AddScore _astop_down_character (Variables|/Game/Blueprints/AIAttributes.AIAttributes_C|GetBitsDropped (Variables|Default|GetAIAttributes)))
    (Actor|DestroyActor)))

(event EventSubtractHealth
  (params (Amount :type Float%20%28single-precision%29))
  (bind _aiattributes (Variables|Default|GetAIAttributes))
  ;[1 1 1] Subtract Health on hit and destroy actor if health <= 0
  (bind _output_get (Variables|/Game/Blueprints/AIAttributes.AIAttributes_C|SetHealth _aiattributes (- (Variables|/Game/Blueprints/AIAttributes.AIAttributes_C|GetHealth _aiattributes) Amount)))
  (CallFunction|KillAI (<= _output_get 0.0)))

(event EventAddHealth
  (params (Amount :type Float%20%28single-precision%29))
  (bind _aiattributes (Variables|Default|GetAIAttributes))
  ;[1 1 1] Add Health Event
  (Variables|/Game/Blueprints/AIAttributes.AIAttributes_C|SetHealth _aiattributes (+ (Variables|/Game/Blueprints/AIAttributes.AIAttributes_C|GetHealth _aiattributes) Amount)))

(event EventBeginPlay)

(fn ConstructionScript)