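; AIAttributes is a Blueprint that holds Health and Shield values, apparently for AI characters.
; Add and subtract functions adjust each value directly, with no clamping and no link between shield and health damage.
; SubtractHealth also returns whether Health has dropped to zero or below, giving callers a death check.
; The event graph is empty, so all changes come from outside callers.
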(event EventBeginPlay)

(event EventTick
  (params (DeltaSeconds :type Float%20%28single-precision%29)))

(fn AddHealth
  (params (AmountToAdd :type Float%20%28single-precision%29))
  (Variables|Default|SetHealth (+ (Variables|Default|GetHealth) AmountToAdd)))

(fn SubtractHealth
  (params (AmountToSubtract :type Float%20%28single-precision%29))
  (bind _output_get (Variables|Default|SetHealth (- (Variables|Default|GetHealth) AmountToSubtract)))
  (return (<= _output_get 0.0)))

(fn AddShield
  (params (AmountToAdd :type Float%20%28single-precision%29))
  (Variables|Default|SetShield (+ (Variables|Default|GetShield) AmountToAdd)))

(fn SubtractShield
  (params (AmountToSubtract :type Float%20%28single-precision%29))
  (Variables|Default|SetShield (- (Variables|Default|GetShield) AmountToSubtract)))