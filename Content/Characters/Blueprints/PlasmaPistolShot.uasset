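; Plasma pistol projectile actor that damages AI characters it overlaps.
; On overlap it spawns the collision effect from its ProjectileAttributes at the SphereCollision location.
; If the other actor casts to AIInterface, it calls SubtractHealth with the projectile's damage.
; The projectile then destroys itself, whatever it hit.
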(event EventBeginPlay)

(event Collision|EventActorBeginOverlap
  (params (OtherActor :type Actor%20Object%20Reference))
  (bind _projectileattributes (Variables|Default|GetProjectileAttributes))
  ;[1 1 1] If projectile overlaps with anything implementing ai interface call subtract health on ai else destroy projectile
  (Effects|SpawnEmitteratLocation (Variables|/Game/Blueprints/ProjectileAttributes.ProjectileAttributes_C|GetBulletCollisionEffect _projectileattributes) (Transformation|GetWorldLocation (Variables|Default|GetSphereCollision self)))
  (bind _asaiinterface (Utilities|Casting|CastToAIInterface OtherActor)
    (:then
      (Default|SubtractHealth _asaiinterface (Variables|/Game/Blueprints/ProjectileAttributes.ProjectileAttributes_C|GetDamage _projectileattributes))
      (Actor|DestroyActor))
    (:CastFailed
      ;;[1 1 1] Collision with something other than enemy
      (Actor|DestroyActor))))

(event EventTick
  (params (DeltaSeconds :type Float%20%28single-precision%29)))

(fn ConstructionScript)